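; Player character with movement and camera input, a health bar widget, and a spell attack fuelled by collected energy orbs.
; CollectEnergy adds orb meshes that Tick swings around the player on a sine-driven orbit, growing their energy and clamped scale over time.
; Orbs within 20 degrees of forward turn red; Fire consumes them, spawning energy-scaled Spell actors and toggling the attack animation flag.
; InflictDamage lowers Health, and Tick derives IsDead from it.
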(event Custom|CollectEnergy
  ;[1 1 1] energy collection
  (Utilities|Array|Add (Variables|Default|GetEnergyArray) 0.0)
  (bind _returnvalue (AddComponent|AddStaticMeshComponent false (Math|Transform|MakeTransform (+ (.location (Transformation|GetRelativeTransform (Variables|Default|GetLoopPosition))) "120.000000, 0, 0") "0, 0, 0" "0.300000,0.300000,0.300000")))
  (Utilities|Array|Add (Variables|Default|GetEnergyMeshes) _returnvalue))

(event EventBeginPlay
  (Utilities|FlowControl|Sequence
    (:then_0
      (Variables|Default|Sethealth (Variables|Default|GetmaxHealth)))
    (:then_1
      (bind _returnvalue (UserInterface|CreateWidget "/Game/UI/HealthBar.HealthBar_C"))
      (bind _output_get (Variables|Default|SethealthBarReference _returnvalue))
      (UserInterface|Viewport|AddtoViewport _output_get 0))))

(event EventTick
  (params (DeltaSeconds :type Float%20%28single-precision%29))
  (bind _energymeshes (Variables|Default|GetEnergyMeshes))
  (Variables|Default|SetdeltaSeconds DeltaSeconds)
  (Utilities|FlowControl|Sequence
    (:then_0
      ;[1 1 1] energy orb rotation
      (for (_array_element _array_index) _energymeshes
        (Transformation|SetRelativeLocation _array_element (Math|Vector|RotateVector (Math|Vector|RotateVector (Math|Vector|MakeVector (+ (.x (Math|Vector|GetForwardVector (Variables|Default|GetLoopPosition))) 3e+02) 0.0 0.0) (Math|Rotator|MakeRotator 0.0 0.0 (+ (* (/ (Math|Conversions|ToFloat(Integer) (+ _array_index 1)) (Math|Conversions|ToFloat(Integer) (Utilities|Array|Length _energymeshes))) 3.6e+02) (* (Math|Trig|Sin(Degrees) (Actor|GetGameTimeSinceCreation)) 8e+03)))) (* (Transformation|GetActorRotation) -1.0)) false false)))
    (:then_1
      ;[1 1 1] energy value growth
      (for (_array_element_2 _array_index_2) (Variables|Default|GetEnergyArray)
        (Utilities|Array|SetArrayElem (Variables|Default|GetEnergyArray) _array_index_2 (+ _array_element_2 (/ (Variables|Default|GetdeltaSeconds) 1e+01)))))
    (:then_2
      ;[1 1 1] energy growth
      (for (_array_element_3 _array_index_3) (Variables|Default|GetEnergyMeshes)
        (Transformation|SetRelativeTransform _array_element_3 (Math|Transform|MakeTransform (.location (Transformation|GetRelativeTransform _array_element_3)) "0, 0, 0" (* "1.000000,1.000000,1.000000" (Math|Float|Clamp(Float) (Utilities|Array|Get(acopy) (Variables|Default|GetEnergyArray) _array_index_3) 0.2 0.5))) false false)))
    (:then_3
      ;[1 1 1] set shootable orb material
      (for _array_element_4 (Variables|Default|GetEnergyMeshes)
        (if (< (Class|KismetMathLibrary|DegAcos (Math|Vector|DotProduct (Math|Vector|Normalize (Math|Vector|GetForwardVector (Transformation|GetActorRotation))) (Math|Vector|Normalize (- (Transformation|GetWorldLocation _array_element_4) (Transformation|GetActorLocation))))) 2e+01)
          (Rendering|Material|SetMaterial _array_element_4 0 "/Game/Materials/Test_Red.Test_Red")
          (else
            (Rendering|Material|SetMaterial _array_element_4 0 "/Game/Shader/Shader/Simple_Shader.Simple_Shader")))))
    (:then_4
      ;[1 1 1] player dies
      (Variables|Default|SetisDead (<= (Variables|Default|Gethealth) 0.0)))))

(event Input|ActionEvents|InputActionFire
  (params (Key :type Key%20Structure :default "None"))
  (:Pressed
    (Utilities|FlowControl|DoOnce false :!label _label
      (:Completed
        ;[1 1 1] shoot orb
        (for (_array_element _array_index) (Variables|Default|GetEnergyMeshes)
          (if (< (Class|KismetMathLibrary|DegAcos (Math|Vector|DotProduct (Math|Vector|Normalize (Math|Vector|GetForwardVector (Transformation|GetActorRotation))) (Math|Vector|Normalize (- (Transformation|GetWorldLocation _array_element) (Transformation|GetActorLocation))))) 2e+01)
            (Components|DestroyComponent _array_element)
            (CallFunction|ShootBullet (Utilities|Array|Get(acopy) (Variables|Default|GetEnergyArray) _array_index))
            (Utilities|Array|RemoveIndex (Variables|Default|GetEnergyMeshes) _array_index)
            (Utilities|Array|RemoveIndex (Variables|Default|GetEnergyArray) _array_index)
            ;[1 1 1] play animation
            (Variables|Default|SetisAttacking true)
            (Utilities|FlowControl|Delay 0.6)
            (Variables|Default|SetisAttacking false))))))
  (:Released
    (goto _label Reset)))

(event Input|AxisEvents|InputAxisForward_Backward
  (params (AxisValue :type Float%20%28single-precision%29))
  ;[1 1 1] character / camera movement
  (Pawn|Input|AddMovementInput (Transformation|GetActorForwardVector) AxisValue false))

(event Input|AxisEvents|InputAxisLeft_right_strafe
  (params (AxisValue :type Float%20%28single-precision%29))
  ;[1 1 1] character / camera movement
  (Pawn|Input|AddMovementInput (Transformation|GetActorRightVector) AxisValue false))

(event Input|AxisEvents|InputAxisLeft_Right_Rotation
  (params (AxisValue :type Float%20%28single-precision%29))
  ;[1 1 1] character / camera movement
  (Pawn|Input|AddControllerYawInput AxisValue))

(event Input|AxisEvents|InputAxisUp_Down_Rotation
  (params (AxisValue :type Float%20%28single-precision%29))
  ;[1 1 1] camera up/down movement
  (Transformation|AddLocalRotation (Variables|Default|GetCamera%20Arm) (Math|Rotator|MakeRotator 0.0 AxisValue 0.0) false false))

(fn ConstructionScript)

(fn ShootBullet
  (params (Energy :type Float%20%28single-precision%29))
  (bind _returnvalue (Math|Float|Clamp(Float) Energy 0.0 0.5))
  (bind _returnvalue_2 (Game|SpawnActorfromClass "/Game/Blueprints/Spell.Spell_C" (Math|Transform|MakeTransform (+ (Transformation|GetActorLocation) (* (Transformation|GetActorForwardVector) 1e+02)) (Transformation|GetActorRotation) (* "30.000000,30.000000,30.000000" _returnvalue)) "Undefined" 0 0))
  (bind _asspell (Utilities|Casting|CastToSpell _returnvalue_2))
  (Variables|/Game/Blueprints/Spell.Spell_C|Setenergy _asspell (* 100 _returnvalue)))

(fn InflictDamage
  (params (Amount :type Float%20%28single-precision%29))
  (Variables|Default|Sethealth (- (Variables|Default|Gethealth) Amount)))
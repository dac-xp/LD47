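; Pickup spawner actor that repeatedly spawns an energy collectible above itself for the lifetime of the level.
; On BeginPlay it plays a lava splash emitter over its spawn area, waits briefly, spawns the pickup, then destroys the emitter.
; The sequence loops after a respawn delay, regardless of whether earlier pickups were collected.
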(event EventBeginPlay
  (bind _returnvalue (Effects|SpawnEmitteratLocation "/Game/InfinityBladeEffects/Effects/FX_Ambient/Fire/P_Lava_Splash_Mesh.P_Lava_Splash_Mesh" (+ (Transformation|GetWorldLocation (Variables|Default|GetSpawnArea)) "0, 0,50.000000") :!label _label))
  (Utilities|FlowControl|Delay 1.0)
  (CallFunction|SpawnPickup)
  (Components|DestroyComponent _returnvalue)
  (Utilities|FlowControl|Delay (Variables|Default|GetRespawnTime))
  (goto _label))

(fn ConstructionScript)

(fn SpawnPickup
  (bind _returnvalue (Game|SpawnActorfromClass "/Game/Blueprints/Collectible_Energy.Collectible_Energy_C" (Math|Conversions|ToTransform(Vector) (+ (Transformation|GetActorLocation) "0, 0,150.000000")) "Undefined" 0 0))
  (return _returnvalue))